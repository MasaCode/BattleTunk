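; AutoMortar_Ver1_2 is a stationary-style auto mortar Blueprint for BattleTank with three barrels on one turret.
; On BeginPlay it initializes its TankAiming component with the three mortar barrels and the turret.
; It then casts its widget component's user widget to HealthBar and sets itself as that bar's tank.
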(event EventBeginPlay
  (Class|TankAimingComponent|InitializewithMultipleBarrel (Variables|Default|GetTankAiming) (Utilities|Array|MakeArray (Variables|Default|GetMortarBarrel) (Variables|Default|GetMortarBarrel2) (Variables|Default|GetMortarBarrel3)) (Variables|Default|GetMortarTurret))
  (CallFunction|InitializeHealthBarWidget))

(fn ConstructionScript)

(fn InitializeHealthBarWidget
  (bind _ashealth_bar (Utilities|Casting|CastToHealthBar (UserInterface|GetUserWidgetObject (Variables|Default|GetWidget))))
  (Variables|/Game/BattleTank/BluePrint/UI/HealthBar.HealthBar_C|SetMyTank _ashealth_bar self))