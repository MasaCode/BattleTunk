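; AutoMortar_Ver1 is an automatic mortar actor for the BattleTank game, built on a tank aiming component with a floating health bar.
; On BeginPlay it hands its mortar barrel and turret to TankAiming for aiming.
; It then casts its widget component to HealthBar and sets itself as that bar's tracked owner.
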(event EventBeginPlay
  (Class|TankAimingComponent|Initialize (Variables|Default|GetTankAiming) (Variables|Default|GetMortarBarrel) (Variables|Default|GetMortarTurret))
  (CallFunction|InitializeHealthBarWidget))

(fn ConstructionScript)

(fn InitializeHealthBarWidget
  (bind _ashealth_bar (Utilities|Casting|CastToHealthBar (UserInterface|GetUserWidgetObject (Variables|Default|GetWidget))))
  (Variables|/Game/BattleTank/BluePrint/UI/HealthBar.HealthBar_C|SetMyTank _ashealth_bar self))