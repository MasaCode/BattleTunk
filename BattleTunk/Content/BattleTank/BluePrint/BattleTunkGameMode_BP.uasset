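; Game mode for BattleTank that tracks the remaining tank count and shows the win and death screens.
; SetTankLeft counts all tanks minus one, fills the player HUD and starts a looping timer that shows the death screen if the player's tank rolls over.
; ChangeTankLeft decrements the count and shows the win screen if the player is alive and the count is one or less.
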(event EventSetTankLeft
  ;[1 1 1] Set Tank Left
  (bind _outactors (Actor|GetAllActorsOfClass "/Script/BattleTunk.Tank"))
  (bind _output_get (Variables|Default|SetTankLeft (- (Utilities|Array|Length _outactors) 1)))
  (bind _foundwidgets (Widget|GetAllWidgetsOfClass "/Game/BattleTank/UI/PlayerUI_BP.PlayerUI_BP_C" true))
  (bind _output_get_2 (Variables|Default|SetPlayerWidget (Utilities|Array|Get(acopy) _foundwidgets)))
  (Default|SetTankLeftText _output_get_2 _output_get)
  (Utilities|Time|SetTimerbyFunctionName self "TankDown" 5.0 true))

(event EventChangeTankLeft
  ;[1 1 1] Change PlayerWidget's Tank Left and decreas tank Left.
  (bind _output_get (Variables|Default|SetTankLeft (- (Variables|Default|GetTankLeft) 1)))
  (Default|SetTankLeftText (Variables|Default|GetPlayerWidget) _output_get)
  (CallFunction|PlayerWin (- (Variables|Default|GetTankLeft) 1)))

(fn ConstructionScript)

(fn CreateUIWidget
  (params (Widget :type User%20Widget%20Class%20Reference))
  (bind _returnvalue (Game|GetPlayerController 0))
  (Viewport|RemoveAllWidgets)
  (bind _returnvalue_2 (UserInterface|CreateWidget Widget _returnvalue))
  (UserInterface|Viewport|AddtoViewport _returnvalue_2 0)
  (Input|SetInputModeUIOnly 0 0 "DoNotLock")
  (Variables|/Script/Engine.PlayerController|SetbShowMouseCursor _returnvalue true))

(fn TankDown
  (bind _returnvalue (Game|GetPlayerController 0))
  (bind _returnvalue_2 (Pawn|GetControlledPawn _returnvalue))
  (if (!= _returnvalue_2 0)
    (if (>= (Math|Float|Absolute(Float) (.roll (Transformation|GetActorRotation _returnvalue_2))) 1.5e+02)
      (CallFunction|CreateUIWidget "/Game/BattleTank/UI/DeathUI_BP.DeathUI_BP_C"))))

(fn PlayerWin
  (params (TankLeft :type Integer))
  (bind _asplayer_tank_controller (Utilities|Casting|CastToPlayerTankController (Game|GetPlayerController 0)))
  (bind _returnvalue (Class|PlayerTankController|IsPlayerAlive _asplayer_tank_controller))
  (if (and _returnvalue (<= TankLeft 0))
    (CallFunction|CreateUIWidget "/Game/BattleTank/UI/WinUI_BP.WinUI_BP_C")))