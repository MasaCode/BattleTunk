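; Tank pawn Blueprint for both player and enemy tanks, colored by material according to IsPlayerTank.
; BeginPlay wires the barrel, turret and tracks into the TankAiming and TankMovement components and links the health bar widget to the tank.
; Input drives track throttles or movement intents, rotates the aiming gimbal and spring arm, and toggles the third-person camera.
; Firing passes through the PlayerTankController's CanFire check, and a separate event plays camera shake.
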(event EventBeginPlay
  ;[1 1 1] Initialize TankAiming, TankMovement and Health Bar Widget
  (Class|TankAimingComponent|Initialize (Variables|Default|GetTankAiming) (Variables|Default|GetBarrel) (Variables|Default|GetTurret))
  (Class|TankMovementComponent|Initialize (Variables|Default|GetTankMovement) (Variables|Default|GetLeft%20Track) (Variables|Default|GetRight%20Track))
  (CallFunction|InitializeHealthBarWidget)
  (if (Variables|Default|GetbIsPlayerTank)
    (CallFunction|SetColor "/Game/BattleTank/BluePrint/Tank/Tank_Nomal/PlayerTank_Material.PlayerTank_Material")
    (else
      (CallFunction|SetColor "/Game/BattleTank/BluePrint/Tank/Tank_Nomal/EnemyTank_Material.EnemyTank_Material"))))

(event EventShakeCamera
  ;[1 1 1] Camera Shake
  (Class|PlayerController|ClientPlayCameraShake (Game|GetPlayerController 0) "/Game/BattleTank/BluePrint/CameraShake_BP.CameraShake_BP_C" 2e+01 "CameraLocal" "0, 0, 0"))

(event Input|ActionEvents|InputActionFire
  (params (Key :type Key%20Structure :default "AnyKey"))
  ;[1 1 1] Firing Input Bind
  (:Pressed
    (bind _asplayer_tank_controller (Utilities|Casting|CastToPlayerTankController (Game|GetPlayerController 0)))
    (bind _returnvalue (Class|PlayerTankController|CanFire _asplayer_tank_controller))
    (if _returnvalue
      (bind _returnvalue_2 (Class|TankAimingComponent|Fire (Variables|Default|GetTankAiming)))
      (if _returnvalue_2
        (Class|PlayerTankController|GetLastFireTime _asplayer_tank_controller)))))

(event Input|ActionEvents|InputActionSwitchCamera
  (params (Key :type Key%20Structure :default "AnyKey"))
  ;[1 1 1] Camera Switch Input Bind
  (:Pressed
    (Components|Activation|ToggleActive (Variables|Default|Get3rd%20Person%20Camera))))

(event Input|AxisEvents|InputAxisAimAzimuth
  (params (AxisValue :type Float%20%28single-precision%29))
  ;[1 1 1] Aiming Input Bind
  (Transformation|AddLocalRotation (Variables|Default|GetAzimuth%20Gimbal) (Math|Rotator|MakeRotator 0.0 0.0 (* AxisValue (Utilities|Time|GetWorldDeltaSeconds) 1e+01)) false false))

(event Input|AxisEvents|InputAxisAimElevation
  (params (AxisValue :type Float%20%28single-precision%29))
  ;[1 1 1] Aiming Input Bind
  (Transformation|AddLocalRotation (Variables|Default|GetSpringArm) (Math|Rotator|MakeRotator 0.0 (* AxisValue (Utilities|Time|GetWorldDeltaSeconds) 1e+01) 0.0) false false))

(event Input|AxisEvents|InputAxisLeftTrackThrottle
  (params (AxisValue :type Float%20%28single-precision%29))
  ;[1 1 1] Movement Input Bind
  (Class|TankTrack|SetThrottle (Variables|Default|GetLeft%20Track) AxisValue))

(event Input|AxisEvents|InputAxisRightTrackThrottle
  (params (AxisValue :type Float%20%28single-precision%29))
  ;[1 1 1] Movement Input Bind
  (Class|TankTrack|SetThrottle (Variables|Default|GetRight%20Track) AxisValue))

(event Input|AxisEvents|InputAxisMoveForward
  (params (AxisValue :type Float%20%28single-precision%29))
  ;[1 1 1] Movement Input Bind
  (Class|TankMovementComponent|IntendMoveForward (Variables|Default|GetTankMovement) AxisValue))

(event Input|AxisEvents|InputAxisTurnRight
  (params (AxisValue :type Float%20%28single-precision%29))
  ;[1 1 1] Movement Input Bind
  (Class|TankMovementComponent|IntendTurnRight (Variables|Default|GetTankMovement) AxisValue))

(fn ConstructionScript)

(fn InitializeHealthBarWidget
  (bind _ashealth_bar (Utilities|Casting|CastToHealthBar (UserInterface|GetUserWidgetObject (Variables|Default|GetHealthBarWidget))))
  (Variables|/Game/BattleTank/BluePrint/UI/HealthBar.HealthBar_C|SetMyTank _ashealth_bar self)
  (if (Variables|Default|GetbIsPlayerTank)
    _))

(fn SetColor
  (params (ColorMaterial :type Material%20Object%20Reference))
  (Rendering|Material|SetMaterial (Variables|Default|GetTank) 0 ColorMaterial)
  (Rendering|Material|SetMaterial (Variables|Default|GetTurret) 0 ColorMaterial)
  (Rendering|Material|SetMaterial (Variables|Default|GetBarrel) 0 ColorMaterial)
  (Rendering|Material|SetMaterial (Variables|Default|GetRight%20Track) 0 ColorMaterial)
  (Rendering|Material|SetMaterial (Variables|Default|GetLeft%20Track) 0 ColorMaterial))